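; Cart actor that rides along the spline of a referenced track when flagged active at BeginPlay.
; A timeline, rate-scaled by Duration and started at CartStartOffset, maps its alpha to distance along the spline, setting world location and rotation.
; ApplyInfluence is an unfinished stub: it loops over components overlapping a pole but applies nothing, leaving its direction and distance math unconnected.
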(event Custom|MoveCart
  (Components|Timeline|SetPlayRate (Variables|Default|GetCartMover) (/ 1.0 (Variables|Default|GetDuration)))
  (Components|Timeline|SetNewTime (Variables|Default|GetCartMover) (Variables|Default|GetCartStartOffset))
  (bind _alpha (Timeline|CartMover Play)
    (:Update
      (Variables|Default|SetAlpha _alpha)
      (Transformation|SetActorLocationAndRotation (Spline|GetLocationatDistanceAlongSpline (Variables|/Game/VehicleAdvBP/Blueprints/SplineCircuit/Track.Track_C|GetSpline (Variables|Default|GetTrackRef)) (Math|Float|Lerp 0.0 (Spline|GetSplineLength (Variables|/Game/VehicleAdvBP/Blueprints/SplineCircuit/Track.Track_C|GetSpline (Variables|Default|GetTrackRef))) (Variables|Default|GetAlpha)) "World") (Spline|GetRotationatDistanceAlongSpline (Variables|/Game/VehicleAdvBP/Blueprints/SplineCircuit/Track.Track_C|GetSpline (Variables|Default|GetTrackRef)) (Math|Float|Lerp 0.0 (Spline|GetSplineLength (Variables|/Game/VehicleAdvBP/Blueprints/SplineCircuit/Track.Track_C|GetSpline (Variables|Default|GetTrackRef))) (Variables|Default|GetAlpha)) "World")))))

(event EventBeginPlay
  (if (Variables|Default|GetActiveCart)
    (CallFunction|MoveCart)))

(fn ConstructionScript)

(fn ApplyInfluence
  (params (L_Pole1 :type Primitive%20Component%20Object%20Reference) (ActionRange :type Primitive%20Component%20Object%20Reference) (MaxDistance :type Float%20%28single-precision%29))
  (LocalVariables|SetL_Pole L_Pole1)
  (LocalVariables|SetL_ActionRange L_Pole1)
  (for _array_element (Class|PrimitiveComponent|GetOverlappingComponents (LocalVariables|GetL_ActionRange))
    (bind _output_get (LocalVariables|SetL_ForeignPole _array_element))
    (if (!= _output_get (LocalVariables|GetL_Pole))
      _)))