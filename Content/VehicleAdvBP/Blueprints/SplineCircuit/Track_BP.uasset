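; Track_BP is a SplineCircuit Blueprint with an unfinished influence step between its static mesh and nearby components.
; On BeginPlay it calls ApplyInfluence with the mesh as the pole and a box as the action range.
; ApplyInfluence loops over components overlapping the box and skips the pole itself, but does nothing with the others.
; Unconnected center-of-mass direction and distance nodes remain, and the construction script is empty.
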(event EventBeginPlay
  (CallFunction|ApplyInfluence (Variables|Default|GetStaticMesh) (Variables|Default|GetBox)))

(fn ConstructionScript)

(fn ApplyInfluence
  (params (Pole :type Primitive%20Component%20Object%20Reference) (ActionRange :type Primitive%20Component%20Object%20Reference))
  (LocalVariables|SetL_Pole Pole)
  (LocalVariables|SetL_ActionRange ActionRange)
  (for _array_element (Class|PrimitiveComponent|GetOverlappingComponents (LocalVariables|GetL_ActionRange))
    (bind _output_get (LocalVariables|SetL_ForeignPole _array_element))
    (if (!= _output_get (LocalVariables|GetL_Pole))
      _)))