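; FloorTile is an endless-track segment that asks VehicleAdvGameMode to add another tile when OutrunTest overlaps its EndTrigger, then destroys itself two seconds later.
; The construction script randomly adds child actors: usually a blocker at one of seven spawn points, otherwise one wandering soul within a box.
; GetAttachTransformed exposes the Arrow's world transform as an attach point.
; SpawnWarp scatters actors in the Warp box but is never called.
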(event OnComponentBeginOverlap(EndTrigger)
  (params (OverlappedComponent :type Primitive%20Component%20Object%20Reference) (OtherActor :type Actor%20Object%20Reference) (OtherComp :type Primitive%20Component%20Object%20Reference) (OtherBodyIndex :type Integer) (bFromSweep :type Boolean) (SweepResult :type Hit%20Result%20Structure%20%28by%20ref%29))
  (Utilities|Casting|CastToOutrunTest OtherActor)
  (bind _asvehicle_adv_game_mode (Utilities|Casting|CastToVehicleAdvGameMode (Game|GetGameMode)))
  (Default|AddFloorTile _asvehicle_adv_game_mode)
  (Utilities|FlowControl|Delay 2.0)
  (Actor|DestroyActor))

(event EventBeginPlay)

(event Collision|EventActorBeginOverlap
  (params (OtherActor :type Actor%20Object%20Reference)))

(event EventTick
  (params (DeltaSeconds :type Float%20%28single-precision%29)))

(fn ConstructionScript
  (CallFunction|SetSpawnPoint)
  (switch int (Math|Random|RandomIntegerinRange 0 2)
    (:Default
      (CallFunction|SpawnBlocker :!label _label))
    (:0
      (goto _label))
    (:1
      (CallFunction|SpawnWanderingSouls))))

(fn GetAttachTransformed
  (return (Transformation|GetWorldTransform (Variables|Default|GetArrow))))

(fn SetSpawnPoint
  (Variables|Default|SetSpawnPoints (Utilities|Array|MakeArray (Transformation|GetRelativeTransform (Variables|Default|GetSpawnPoint)) (Transformation|GetRelativeTransform (Variables|Default|GetSpawnPointL)) (Transformation|GetRelativeTransform (Variables|Default|GetSpawnPointR)) (Transformation|GetRelativeTransform (Variables|Default|GetSpawnPointR1)) (Transformation|GetRelativeTransform (Variables|Default|GetSpawnPointL1)) (Transformation|GetRelativeTransform (Variables|Default|GetSpawnPoint1)) (Transformation|GetRelativeTransform (Variables|Default|GetSpawnPoint2)))))

(fn SpawnBlocker
  (bind _spawnpoints (Variables|Default|GetSpawnPoints))
  (AddComponent|AddChildActorComponent false (Utilities|Array|Get(acopy) _spawnpoints (Math|Random|RandomIntegerinRange 0 (Utilities|Array|LastIndex _spawnpoints)))))

(fn SpawnWanderingSouls
  (bind _wandering_soul (Variables|Default|GetWandering%20soul))
  (for _index (range 0 0)
    (AddComponent|AddChildActorComponent false (Math|Conversions|ToTransform(Vector) (Math|Random|RandomPointinBoundingBox (Variables|/Script/Engine.SceneComponent|GetRelativeLocation _wandering_soul) (Variables|/Script/Engine.BoxComponent|GetBoxExtent _wandering_soul))))))

(fn SpawnWarp
  (bind _warp (Variables|Default|GetWarp))
  (for _index (range 0 5)
    (AddComponent|AddChildActorComponent false (Math|Conversions|ToTransform(Vector) (Math|Random|RandomPointinBoundingBox (Variables|/Script/Engine.SceneComponent|GetRelativeLocation _warp) (Variables|/Script/Engine.BoxComponent|GetBoxExtent _warp))))))