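; WanderingSoul is a collectible actor that rewards the overlapping OutrunTest or NormalTest object with score and health, then destroys itself.
; Its capsule overlap event casts to OutrunTest first, then NormalTest, and edits that object's variables directly.
; NormalTest gets a smaller heal capped at 100 and also an integer score increase, while OutrunTest's heal is uncapped here.
; The Blueprint contains no movement or AI logic.
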(event OnComponentBeginOverlap(Capsule)
  (params (OverlappedComponent :type Primitive%20Component%20Object%20Reference) (OtherActor :type Actor%20Object%20Reference) (OtherComp :type Primitive%20Component%20Object%20Reference) (OtherBodyIndex :type Integer) (bFromSweep :type Boolean) (SweepResult :type Hit%20Result%20Structure%20%28by%20ref%29))
  (bind _asoutrun_test (Utilities|Casting|CastToOutrunTest OtherActor)
    (:then
      (Actor|DestroyActor)
      (Variables|/Game/VehicleAdvBP/Blueprints/OutrunTest.OutrunTest_C|SetScore _asoutrun_test (+ (Variables|/Game/VehicleAdvBP/Blueprints/OutrunTest.OutrunTest_C|GetScore _asoutrun_test) 1e+01))
      (Variables|/Game/VehicleAdvBP/Blueprints/OutrunTest.OutrunTest_C|SetHP _asoutrun_test (+ (Variables|/Game/VehicleAdvBP/Blueprints/OutrunTest.OutrunTest_C|GetHP _asoutrun_test) 25.0)))
    (:CastFailed
      (bind _asnormal_test (Utilities|Casting|CastToNormalTest OtherActor))
      (Actor|DestroyActor)
      (Variables|/Game/VehicleAdvBP/Blueprints/NormalTest.NormalTest_C|SetScoreInteger _asnormal_test (+ (Variables|/Game/VehicleAdvBP/Blueprints/NormalTest.NormalTest_C|GetScoreInteger _asnormal_test) 10))
      (Variables|/Game/VehicleAdvBP/Blueprints/NormalTest.NormalTest_C|SetScore _asnormal_test (+ (Variables|/Game/VehicleAdvBP/Blueprints/NormalTest.NormalTest_C|GetScore _asnormal_test) 1e+01))
      (Variables|/Game/VehicleAdvBP/Blueprints/NormalTest.NormalTest_C|SetHP _asnormal_test (+ (Variables|/Game/VehicleAdvBP/Blueprints/NormalTest.NormalTest_C|GetHP _asnormal_test) 1e+01))
      (if (> (Variables|/Game/VehicleAdvBP/Blueprints/NormalTest.NormalTest_C|GetHP _asnormal_test) 1e+02)
        (Variables|/Game/VehicleAdvBP/Blueprints/NormalTest.NormalTest_C|SetHP _asnormal_test 1e+02)))))

(event EventBeginPlay)

(event Collision|EventActorBeginOverlap
  (params (OtherActor :type Actor%20Object%20Reference)))

(event EventTick
  (params (DeltaSeconds :type Float%20%28single-precision%29)))

(fn ConstructionScript)